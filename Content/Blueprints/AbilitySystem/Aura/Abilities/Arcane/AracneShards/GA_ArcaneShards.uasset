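; Arcane Shards gameplay ability that shows a magic circle, waits for an input press, then places a series of points at the location under the mouse.
; A temporary point collection actor supplies ground points with random yaw at that impact point.
; A looping timer steps through them, currently drawing only debug spheres as shard placeholders.
; After the last point, it clears the timer, destroys the collection and ends the ability.
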(event `self.K2_ActivateAbility`
  (`|ExecutionSequence`
    (:`then_0`
      (message `PlayerInterface.ShowMagicCircle` (`self.GetAvatarActorFromActorInfo`) null))
    (:`then_1`
      (`AbilityTask_WaitInputPress.WaitInputPress` false
        (:`OnPress`
          (bind (_asynctaskproxy _datahandle) (`TargetDataUnderMouse.CreateTargetDataUnderMouse`)
            (:`ValidData`
              (bind (_bblockinghit _binitialoverlap _time _distance _location _impactpoint) (`GameplayStatics.BreakHitResult` (`AbilitySystemBlueprintLibrary.GetHitResultFromTargetData` _datahandle)))
              (bind _returnvalue (`|SpawnActorFromClass` "/Game/Blueprints/AbilitySystem/Aura/Abilities/Arcane/AracneShards/BP_PointCollection.BP_PointCollection_C" (`KismetMathLibrary.MakeTransform` _impactpoint) "AlwaysSpawn" "MultiplyWithRoot" null null))
              (bind _output_get (set `self.PointCollection` _returnvalue))
              (set `self.GroundPoints` (`PointCollection.GetGroundPoints` _output_get _impactpoint (`self.NumPoints`) (`KismetMathLibrary.RandomFloatInRange` 0.0 360.0)))
              (bind _returnvalue_2 (`KismetSystemLibrary.K2_SetTimerDelegate` (delegate `SpawnShard`) (`self.ShardSpawnDeltaTime`) true))
              (set `self.ShardSpawnTimer` _returnvalue_2)
              (`self.SpawnShard`)
              (message `PlayerInterface.HideMagicCircle` (`self.GetAvatarActorFromActorInfo`)))))))))

(event `SpawnShard`
  (if (< (`self.Count`) (`self.NumPoints`))
    (`KismetSystemLibrary.DrawDebugSphere` (`SceneComponent.K2_GetComponentLocation` (`|GetArrayItem` (`self.GroundPoints`) (`self.Count`))) 20.0 12 (struct :`R` 1.0 :`G` 1.0 :`B` 1.0 :`A` 1.0) 20.0)
    (`/Engine/EditorBlueprintResources/StandardMacros.IncrementInt` (`self.Count`))
    (else
      (`KismetSystemLibrary.K2_ClearAndInvalidateTimerHandle` (`self.ShardSpawnTimer`))
      (`KismetSystemLibrary.Delay` 0.2)
      (`Actor.K2_DestroyActor` (`self.PointCollection`))
      (`self.K2_EndAbility`))))